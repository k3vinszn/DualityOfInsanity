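; BP_Balança is a scale that acts as a two-key lock for a linked door.
; Its Hit event checks the colliding actor's class, setting a separate flag for BP_Key and BP_Key_1, with no reset.
; Once both flags are set, a DoOnce calls OpenDoor on the referenced door and plays the DoorOpen sound event at that door's location.
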(event `self.ReceiveHit`
  (params (MyComp :type "PrimitiveComponent Object Reference") (Other :type "Actor Object Reference") (OtherComp :type "PrimitiveComponent Object Reference") (bSelfMoved :type Boolean) (HitLocation :type "Vector Structure") (HitNormal :type "Vector Structure") (NormalImpulse :type "Vector Structure") (Hit :type "HitResult Structure (by ref)"))
  (bind _returnvalue (`GameplayStatics.GetObjectClass` Other))
  (`|ExecutionSequence`
    (:`then_0`
      (if (== _returnvalue "/Game/BP_Key_1.BP_Key_1_C")
        (set `self.keyPlaced2` true)))
    (:`then_1`
      (if (== _returnvalue "/Game/BP_Key.BP_Key_C")
        (set `self.keyPlaced` true)))
    (:`then_2`
      (if (and (`self.keyPlaced`) (`self.keyPlaced2`))
        (`/Engine/EditorBlueprintResources/StandardMacros.DoOnce` false
          (:`Completed`
            (`/Game/Door/BP_Door.OpenDoor` (`self.doorVar`))
            (`FMODBlueprintStatics.PlayEventAtLocation` "/Game/FMOD/Events/SFX/DoorOpen.DoorOpen" (`KismetMathLibrary.Conv_VectorToTransform` (`self.K2_GetActorLocation` (`self.doorVar`))))))))))

(fn `UserConstructionScript`)