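; BP_ItemCollectable3 is an item actor that shows an on-screen widget while the first-person character is inside its box trigger.
; Entering the box creates BP_widget7 and adds it to the viewport, guarded by a DoOnce.
; Leaving calls the widget's fade-out, removes it immediately afterwards and resets the guard.
; Pressing F only removes the widget; no collection or progress-bar logic appears here.
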(event `self.Box.OnComponentBeginOverlap`
  (params (OverlappedComponent :type "PrimitiveComponent Object Reference") (OtherActor :type "Actor Object Reference") (OtherComp :type "PrimitiveComponent Object Reference") (OtherBodyIndex :type Integer) (bFromSweep :type Boolean) (SweepResult :type "HitResult Structure (by ref)"))
  (bind _asbp_first_person_character (cast `/Game/FirstPerson/Blueprints/BP_FirstPersonCharacter` OtherActor))
  (set `self.First Person BP` _asbp_first_person_character)
  (if (== OtherActor (`self.First Person BP`))
    (`/Engine/EditorBlueprintResources/StandardMacros.DoOnce` false :!label _label
      (:`Completed`
        (bind _returnvalue (`|CreateWidget` "/Game/Pensamentos/Pensamento7/BP_widget7.BP_widget7_C" (`GameplayStatics.GetPlayerController` 0)))
        (bind _output_get (set `self.HUD 7 widget` _returnvalue))
        (`UserWidget.AddToViewport` _output_get 0)))))

(event `self.Box.OnComponentEndOverlap`
  (params (OverlappedComponent :type "PrimitiveComponent Object Reference") (OtherActor :type "Actor Object Reference") (OtherComp :type "PrimitiveComponent Object Reference") (OtherBodyIndex :type Integer))
  (cast `/Game/FirstPerson/Blueprints/BP_FirstPersonCharacter` OtherActor)
  (`/Game/Pensamentos/Pensamento7/BP_widget7.FadeOutWidget` (`self.HUD 7 widget`))
  (`Widget.RemoveFromParent` (`self.HUD 7 widget`))
  (goto _label :!via `Reset`))

(event `Key|F`
  (params (Key :type "Key Structure"))
  (:`Pressed`
    (`Widget.RemoveFromParent` (`self.HUD 7 widget`))))

(fn `UserConstructionScript`)