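; BP_ItemCollectable2 is an item actor that shows a BP_widget7insane HUD widget while the first-person character is inside its Box trigger.
; Begin overlap creates the widget and adds it to the viewport through a DoOnce, which end overlap resets.
; End overlap calls FadeOut and removes the widget immediately afterwards.
; Pressing F only removes the widget; this Blueprint holds no collection logic.
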(event `self.Box.OnComponentBeginOverlap`
  (params (OverlappedComponent :type "PrimitiveComponent Object Reference") (OtherActor :type "Actor Object Reference") (OtherComp :type "PrimitiveComponent Object Reference") (OtherBodyIndex :type Integer) (bFromSweep :type Boolean) (SweepResult :type "HitResult Structure (by ref)"))
  (bind _asbp_first_person_character (cast `/Game/FirstPerson/Blueprints/BP_FirstPersonCharacter` OtherActor))
  (set `self.BP first Person` _asbp_first_person_character)
  (if (== OtherActor (`self.BP first Person`))
    (`/Engine/EditorBlueprintResources/StandardMacros.DoOnce` false :!label _label
      (:`Completed`
        (bind _returnvalue (`|CreateWidget` "/Game/Pensamentos/Pensamento7/BP_widget7insane.BP_widget7insane_C" (`GameplayStatics.GetPlayerController` 0)))
        (bind _output_get (set `self.HUD widget 7 insane` _returnvalue))
        (`UserWidget.AddToViewport` _output_get 0)))))

(event `self.Box.OnComponentEndOverlap`
  (params (OverlappedComponent :type "PrimitiveComponent Object Reference") (OtherActor :type "Actor Object Reference") (OtherComp :type "PrimitiveComponent Object Reference") (OtherBodyIndex :type Integer))
  (cast `/Game/FirstPerson/Blueprints/BP_FirstPersonCharacter` OtherActor)
  (`/Game/Pensamentos/Pensamento7/BP_widget7insane.FadeOut` (`self.HUD widget 7 insane`))
  (`Widget.RemoveFromParent` (`self.HUD widget 7 insane`))
  (goto _label :!via `Reset`))

(event `Key|F`
  (params (Key :type "Key Structure"))
  (:`Pressed`
    (`Widget.RemoveFromParent` (`self.HUD widget 7 insane`))))

(fn `UserConstructionScript`)